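; BP_Board is a shooting-gallery target that adds score for Center or Side hits and deducts a point when it expires unhit.
; Either outcome spawns a replacement at a random point inside the tagged AreaBoundry trigger box, unless time is over, then destroys the board.
; Tick uses the player controller's Timer to select no movement, horizontal or vertical movement, with randomized starting direction and reversal at the boundary edges.
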(event EventBeginPlay
  (bind _asmy_player_controller (Utilities|Casting|CastToMyPlayerController (Game|GetPlayerController 0)))
  (Variables|Default|SetAs%20My%20Player%20Controller _asmy_player_controller)
  ;[1 1 1] Get Area Boundry
  (bind _outactors (Actor|GetAllActorsOfClasswithTag "/Script/Engine.TriggerBox" "AreaBoundry"))
  (for _array_element _outactors
    (Variables|Default|SetAreaBoundry _array_element))
  ;[1 0.1647 0] Auto Destroy
  (Utilities|FlowControl|Delay (Variables|Default|GetDestroyInSeconds))
  (CallFunction|ManageScore -1)
  (CallFunction|SpawnBoard)
  (Actor|DestroyActor))

(event EventTick
  (params (DeltaSeconds :type Float%20%28single-precision%29))
  (bind _returnvalue (Transformation|GetActorLocation))
  (bind _returnvalue_2 (Transformation|GetActorLocation))
  (bind _areaboundry (Variables|Default|GetAreaBoundry))
  (bind _as_my_player_controller (Variables|Default|GetAs%20My%20Player%20Controller))
  (bind _areaboundry_2 (Variables|Default|GetAreaBoundry))
  (bind (_origin _boxextent) (Collision|GetActorBounds _areaboundry false false))
  (bind (_origin_2 _boxextent_2) (Collision|GetActorBounds _areaboundry_2 false false))
  (bind _timer (Variables|/Game/FirstPersonBP/Blueprints/MyPlayerController.MyPlayerController_C|GetTimer _as_my_player_controller))
  ;[0.07292 0.07292 0.07292] Board Movement
  (if (not (>= _timer 40))
    ;;[1 1 1] Movement Randomization
    (if (Variables|Default|GetRandomized)
      _
      (else
        (if (Math|Random|RandomBool)
          _
          (else
            (Math|Float|NegateFloat (Variables|Default|GetSpeedVertical)
              (:%20%20
                (Math|Float|NegateFloat (Variables|Default|GetSpeedHorizontal)
                  (:%20%20
                    _))))))
        (Variables|Default|SetRandomized true)))
    (if (>= _timer 20)
      ;;[1 1 1] Horizontal Movement
      (Transformation|AddActorWorldOffset (Math|Vector|MakeVector 0.0 (* DeltaSeconds (Variables|Default|GetSpeedHorizontal)) 0.0))
      (if (or (<= (.y _returnvalue) (.y (- _origin _boxextent))) (>= (.y _returnvalue) (.y (+ _origin _boxextent))))
        (Math|Float|NegateFloat (Variables|Default|GetSpeedHorizontal)))
      (else
        ;;[1 1 1] Vertical Movement
        (Transformation|AddActorWorldOffset (Math|Vector|MakeVector 0.0 0.0 (* DeltaSeconds (Variables|Default|GetSpeedVertical))))
        (if (or (<= (.z _returnvalue_2) (.z (- _origin_2 _boxextent_2))) (>= (.z _returnvalue_2) (.z (+ _origin_2 _boxextent_2))))
          (Math|Float|NegateFloat (Variables|Default|GetSpeedVertical)))))))

(event EventShoot
  (params (HitResult :type Hit%20Result%20Structure))
  (bind _spawndelay (Variables|Default|GetSpawnDelay))
  ;[1 0 0] Board Hit Events
  ;;[0 0 0] Center
  (if (== (Variables|Default|GetCenter) (.hitcomponent HitResult))
    (CallFunction|ManageScore 2)
    (Rendering|SetActorHiddenInGame true)
    (Collision|SetActorEnableCollision false)
    (Utilities|FlowControl|Delay _spawndelay)
    (CallFunction|SpawnBoard)
    (Actor|DestroyActor)
    (else
      ;;[0 0 0] Side
      (if (== (Variables|Default|GetSide) (.hitcomponent HitResult))
        (CallFunction|ManageScore 1)
        (Rendering|SetActorHiddenInGame true)
        (Collision|SetActorEnableCollision false)
        (Utilities|FlowControl|Delay _spawndelay)
        (CallFunction|SpawnBoard)
        (Actor|DestroyActor)))))

(fn ConstructionScript)

(fn ManageScore
  (params (Increment :type Integer))
  (bind _as_my_player_controller (Variables|Default|GetAs%20My%20Player%20Controller))
  (Variables|/Game/FirstPersonBP/Blueprints/MyPlayerController.MyPlayerController_C|SetScore _as_my_player_controller (+ (Variables|/Game/FirstPersonBP/Blueprints/MyPlayerController.MyPlayerController_C|GetScore _as_my_player_controller) Increment)))

(fn SpawnBoard
  (bind _areaboundry (Variables|Default|GetAreaBoundry))
  (bind (_origin _boxextent) (Collision|GetActorBounds _areaboundry false false))
  (bind _returnvalue (- _origin _boxextent))
  (bind _returnvalue_2 (+ _origin _boxextent))
  (if (not (Variables|/Game/FirstPersonBP/Blueprints/MyPlayerController.MyPlayerController_C|GetTimeOver (Variables|Default|GetAs%20My%20Player%20Controller)))
    (Game|SpawnActorfromClass "BP_Board_C" (Math|Transform|MakeTransform (Math|Vector|MakeVector (Math|Random|RandomFloatinRange (.x _returnvalue) (.x _returnvalue_2)) (Math|Random|RandomFloatinRange (.y _returnvalue) (.y _returnvalue_2)) (Math|Random|RandomFloatinRange (.z _returnvalue) (.z _returnvalue_2))) "0,90.000000, 0" "1,1,1") "Undefined" 0 0)))