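; BP_StartBoard is a start target that begins a timed, scored round when its Shoot event fires.
; Shoot hides the board, destroys a BP_StartDummy if present, then after a short delay spawns an actor at a randomized X/Y position and fixed height.
; It then starts and resets the timer, time-over flag and score on MyPlayerController before destroying itself.
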(event EventShoot
  (params (HitResult :type Hit%20Result%20Structure))
  ;[1 0 0] Triggered & Destroy
  (Rendering|SetActorHiddenInGame true)
  (bind _returnvalue (Actor|GetActorOfClass "/Game/Blueprints/BP_StartDummy.BP_StartDummy_C"))
  (Utilities|IsValid _returnvalue
    (:Is%20Valid
      (Actor|DestroyActor _returnvalue))
    (:Is%20Not%20Valid
      _))
  ;[0 1 0] Spawn Board
  (Utilities|FlowControl|Delay 1.0)
  (Game|SpawnActorfromClass "/Game/Blueprints/BP_Board.BP_Board_C" (Math|Transform|MakeTransform (Math|Vector|MakeVector (Math|Random|RandomFloatinRange 6.5e+02 1.5e+03) (Math|Random|RandomFloatinRange -3.5e+02 3.5e+02) 2.5e+02) "0,90.000000, 0" "1,1,1") "Undefined" 0 0)
  ;[0 0 1] Reset Settings
  (bind _asmy_player_controller (Utilities|Casting|CastToMyPlayerController (Game|GetPlayerController 0)))
  (Variables|/Game/FirstPersonBP/Blueprints/MyPlayerController.MyPlayerController_C|SetTimerStart _asmy_player_controller true)
  (Variables|/Game/FirstPersonBP/Blueprints/MyPlayerController.MyPlayerController_C|SetTimer _asmy_player_controller 60)
  (Variables|/Game/FirstPersonBP/Blueprints/MyPlayerController.MyPlayerController_C|SetTimeOver _asmy_player_controller false)
  (Variables|/Game/FirstPersonBP/Blueprints/MyPlayerController.MyPlayerController_C|SetScore _asmy_player_controller 0)
  (Actor|DestroyActor))

(fn ConstructionScript)