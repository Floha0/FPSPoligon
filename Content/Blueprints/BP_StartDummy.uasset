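; BP_StartDummy is a shootable start target that begins a timed scoring round.
; When shot, it plays a dissolve Niagara effect, hides its mesh and disables collision.
; After a short delay it spawns a BP_Dummy at a randomized floor position, resets timer and score on MyPlayerController, then destroys itself.
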(event EventShoot
  (params (HitResult :type Hit%20Result%20Structure))
  ;[1 0 0] Trigger & Destroy
  (Components|Activation|SetActive (Variables|Default|GetNS_Disslove) true true)
  (Development|SetHiddeninGame (Variables|Default|GetSkeletalMesh) true false)
  (Collision|SetActorEnableCollision false)
  ;[0 1 0] Spawn Dummy
  (Utilities|FlowControl|Delay 2.0)
  (Game|SpawnActorfromClass "/Game/Blueprints/BP_Dummy.BP_Dummy_C" (Math|Transform|MakeTransform (Math|Vector|MakeVector (Math|Random|RandomFloatinRange 6.5e+02 1.5e+03) (Math|Random|RandomFloatinRange -3.5e+02 3.5e+02) (.z (Transformation|GetWorldLocation (Variables|Default|GetSkeletalMesh)))) "0,90.000000, 0" "1,1,1") "Undefined" 0 0)
  ;[0 0 1] Reset Settings
  (bind _asmy_player_controller (Utilities|Casting|CastToMyPlayerController (Game|GetPlayerController 0)))
  (Variables|/Game/FirstPersonBP/Blueprints/MyPlayerController.MyPlayerController_C|SetTimer _asmy_player_controller 60)
  (Variables|/Game/FirstPersonBP/Blueprints/MyPlayerController.MyPlayerController_C|SetTimerStart _asmy_player_controller true)
  (Variables|/Game/FirstPersonBP/Blueprints/MyPlayerController.MyPlayerController_C|SetTimeOver _asmy_player_controller false)
  (Variables|/Game/FirstPersonBP/Blueprints/MyPlayerController.MyPlayerController_C|SetScore _asmy_player_controller 0)
  (Utilities|FlowControl|Delay 3.5)
  (Actor|DestroyActor))

(fn ConstructionScript)