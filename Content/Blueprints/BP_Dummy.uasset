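; BP_Dummy is a shooting target that adjusts the player's score and spawns its own replacement until time runs out.
; A Shoot event scores headshots higher than other hits, plays a matching dissolve effect, hides the mannequin and disables collision.
; After a delay it spawns a new dummy at a random position and destroys only the mesh component.
; An unhit dummy times out, costing a point, respawning and destroying itself.
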(event EventShoot
  (params (HitResult :type Hit%20Result%20Structure))
  (bind _spawndelay (Variables|Default|GetSpawnDelay))
  ;[1 0 0] Dummy Hit Events
  (if (Utilities|Name|Equal(Name) (.hitbonename HitResult) "Head")
    ;;[0 0 0] Head
    (Variables|Default|SetIsAlive false)
    (CallFunction|Death (Variables|Default|GetNS_Disslove2))
    (CallFunction|ManageScore 2)
    (Utilities|FlowControl|Delay _spawndelay)
    (CallFunction|SpawnDummy)
    (Components|DestroyComponent (Variables|Default|GetMannequinSK))
    (else
      ;;[0 0 0] Body
      (Variables|Default|SetIsAlive false)
      (CallFunction|Death (Variables|Default|GetNS_Disslove))
      (CallFunction|ManageScore 1)
      (Utilities|FlowControl|Delay _spawndelay)
      (CallFunction|SpawnDummy)
      (Components|DestroyComponent (Variables|Default|GetMannequinSK)))))

(event EventBeginPlay
  (bind _asmy_player_controller (Utilities|Casting|CastToMyPlayerController (Game|GetPlayerController 0)))
  (Variables|Default|SetAs%20My%20Player%20Controller _asmy_player_controller)
  ;[1 0.1651 0] AutoDestroy
  (Utilities|FlowControl|Delay (Variables|Default|GetDestroyInSeconds))
  (if (Variables|Default|GetIsAlive)
    (CallFunction|ManageScore -1)
    (CallFunction|SpawnDummy)
    (Actor|DestroyActor)))

(fn ConstructionScript)

(fn Death
  (params (DeathVFX :type Niagara%20Component%20Object%20Reference))
  (Components|Activation|SetActive DeathVFX true true)
  (Development|SetHiddeninGame (Variables|Default|GetMannequinSK) true false)
  (Collision|SetActorEnableCollision false))

(fn ManageScore
  (params (Increment :type Integer))
  (bind _as_my_player_controller (Variables|Default|GetAs%20My%20Player%20Controller))
  (Variables|/Game/FirstPersonBP/Blueprints/MyPlayerController.MyPlayerController_C|SetScore _as_my_player_controller (+ (Variables|/Game/FirstPersonBP/Blueprints/MyPlayerController.MyPlayerController_C|GetScore _as_my_player_controller) Increment)))

(fn SpawnDummy
  (if (not (Variables|/Game/FirstPersonBP/Blueprints/MyPlayerController.MyPlayerController_C|GetTimeOver (Variables|Default|GetAs%20My%20Player%20Controller)))
    (Game|SpawnActorfromClass "BP_Dummy_C" (Math|Transform|MakeTransform (Math|Vector|MakeVector (Math|Random|RandomFloatinRange 6.5e+02 1.5e+03) (Math|Random|RandomFloatinRange -3.5e+02 3.5e+02) 1.7e+02) "0,90.000000, 0" "1,1,1") "Undefined" 0 0)))